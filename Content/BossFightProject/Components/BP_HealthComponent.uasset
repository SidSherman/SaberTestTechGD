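; BP_HealthComponent is a health component that tracks an owner's HP and death state in the boss fight project.
; It fills current HP to max on BeginPlay, and the ChangeHP event applies a signed delta clamped between zero and max while alive.
; Each change fires the OnChangeHP dispatcher; reaching zero sets IsDead, fires OnDeath and prints a debug string.
; Simple getters expose HP and death state.
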(event `self.ReceiveBeginPlay`
  ;[1 1 1] Set Current HP on BeginPlay
  (set `self.CurrenHP` (`self.MaxHP`)))

(event `ChangeHP`
  (params (DeltaHP :type "Float (double-precision)"))
  ;[1 1 1] HP Changing Event
  ;;[1 1 1] Check Character dead or alive
  (if (not (`self.bIsDead`))
    ;;[1 1 1] ChangeHP
    (bind _output_get (set `self.CurrenHP` (`KismetMathLibrary.FClamp` (+ DeltaHP (`self.CurrenHP`)) 0.0 (`self.MaxHP`))))
    (`self.OnChangeHP` (`self.MaxHP`) _output_get)
    ;;[1 1 1] Check Should character to be dead after HP changing
    (if (<= _output_get 0.0)
      (`self.SetIsDead` true)
      (`self.OnDeath`)
      (`KismetSystemLibrary.PrintString` "death"))))

(fn `GetCurrentHP`
  (returns (CurrenHP :type "Float (double-precision)"))
  (return (`self.CurrenHP`)))

(fn `GetIsDead`
  (returns (bIsDead :type Boolean))
  (return (`self.bIsDead`)))

(fn `GetMaxHP`
  (returns (MaxHP :type "Float (double-precision)"))
  (return (`self.MaxHP`)))

(fn `SetIsDead`
  (params (bIsDead :type Boolean))
  (set `self.bIsDead` bIsDead))