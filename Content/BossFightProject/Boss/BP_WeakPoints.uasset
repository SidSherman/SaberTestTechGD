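; BP_WeakPoints is a boss weak point actor with its own health that can be switched on and off.
; Activation toggles sphere collision and fades the mesh material's Emission through a timeline.
; Damage not instigated by its owner reduces health, broadcasts OnDamage, and plays an impact sound with an emission flash.
; At zero health it spawns sparks, plays a sound and destroys itself.
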(event `/Game/BossFightProject/Boss/BPI_WeakPoint.Init`
  (params (Health :type "Float (double-precision)"))
  (set `self.Health` Health))

(event `/Game/BossFightProject/Boss/BPI_WeakPoint.ActivatePoint`
  (set `self.bIsActive` true)
  (`PrimitiveComponent.SetCollisionEnabled` (`self.Sphere`) "QueryOnly")
  (bind (_direction _alpha) (`Timeline|Timeline` :!label _label)
    (:`Update`
      (`MeshComponent.SetScalarParameterValueOnMaterials` (`self.Mesh`) "Emission" _alpha))))

(event `/Game/BossFightProject/Boss/BPI_WeakPoint.DeactivatePoint`
  (set `self.bIsActive` false)
  (`PrimitiveComponent.SetCollisionEnabled` (`self.Sphere`) "NoCollision")
  (goto _label :!via `ReverseFromEnd`))

(event `DestroyPoint`
  (bind _returnvalue (`SceneComponent.K2_GetComponentLocation` (`self.Mesh`)))
  (`GameplayStatics.SpawnEmitterAtLocation` "/Game/Dev/ContentToDelete/Realistic_Starter_VFX_Pack_Vol2/Particles/Explosion/P_Explosion_Sparcle.P_Explosion_Sparcle" _returnvalue)
  (`GameplayStatics.PlaySoundAtLocation` "/Game/Dev/ContentToDelete/Weapon/MilitaryWeapDark/Sound/Shotgun/Shotgun_ImpactBody_Cue.Shotgun_ImpactBody_Cue" _returnvalue (struct) 1.0 1.0 0.0 null null null null)
  (`self.K2_DestroyActor`))

(event `self.ReceiveAnyDamage`
  (params (Damage :type "Float (single-precision)") (DamageType :type "DamageType Object Reference") (InstigatedBy :type "Controller Object Reference") (DamageCauser :type "Actor Object Reference"))
  (bind _returnvalue (`Controller.K2_GetPawn` InstigatedBy))
  (`/Engine/EditorBlueprintResources/StandardMacros.IsValid` InstigatedBy
    (:`Is Valid`
      (`/Engine/EditorBlueprintResources/StandardMacros.IsValid` _returnvalue
        (:`Is Valid`
          (if (!= _returnvalue (`self.GetOwner`))
            (bind _output_get (set `self.Health` (- (`self.Health`) Damage) :!label _label_2))
            (`self.OnDamage` Damage)
            (if (<= _output_get 0.0)
              (`self.DestroyPoint`)
              (else
                (`GameplayStatics.PlaySoundAtLocation` "/Game/Dev/ContentToDelete/Weapon/MilitaryWeapDark/Sound/Rifle/Rifle_ImpactBody_Cue.Rifle_ImpactBody_Cue" (`SceneComponent.K2_GetComponentLocation` (`self.Mesh`)) (struct) 1.0 1.0 0.0 null null null null)
                (bind (_direction _alpha) (`Timeline|Timeline_0` :!via `PlayFromStart`)
                  (:`Update`
                    (`MeshComponent.SetScalarParameterValueOnMaterials` (`self.Mesh`) "Emission" _alpha)))))))))
    (:`Is Not Valid`
      (goto _label_2))))

(fn `UserConstructionScript`)