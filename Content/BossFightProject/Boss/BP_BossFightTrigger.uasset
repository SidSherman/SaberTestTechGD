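; BP_BossFightTrigger is a level trigger that starts a boss fight when the player enters it and seals the arena.
; On the first overlap by an actor tagged Player, it sets that actor as the Boss target, starts combat, closes the Door and notifies BP_BossGameState.
; It opens the Door on BeginPlay and again when the boss health component's OnDeath event fires.
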(event `self.ReceiveActorBeginOverlap`
  (params (OtherActor :type "Actor Object Reference"))
  (bind _boss (`self.Boss`))
  (`/Engine/EditorBlueprintResources/StandardMacros.IsValid` OtherActor
    (:`Is Valid`
      (if (`self.ActorHasTag` OtherActor "Player")
        (if (not (`self.bIsActive`))
          (set `self.bIsActive` true)
          (`/Game/BossFightProject/Boss/BP_Boss.SetTarget` _boss OtherActor)
          (`/Game/BossFightProject/Boss/BP_Boss.StartCombat` _boss)
          (`/Game/BossFightProject/Core/BP_Door.Close` (`self.Door`))
          (bind _asbp_boss_game_state (cast `/Game/BossFightProject/Core/BP_BossGameState` (`GameplayStatics.GetGameState`)))
          (`/Game/BossFightProject/Core/BP_BossGameState.BossActive` _asbp_boss_game_state))))))

(event `self.ReceiveBeginPlay`
  (add `/Game/BossFightProject/Components/BP_HealthComponent.OnDeath` (`/Game/BossFightProject/Boss/BP_Boss.BP_HealthComponent` (`self.Boss`)) (delegate `OnDeath_Event`))
  (`/Game/BossFightProject/Core/BP_Door.Open` (`self.Door`)))

(event `OnDeath_Event`
  (`/Game/BossFightProject/Core/BP_Door.Open` (`self.Door`)))

(fn `UserConstructionScript`)