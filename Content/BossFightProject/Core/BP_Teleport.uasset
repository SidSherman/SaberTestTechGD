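; BP_Teleport is a linked teleporter that moves the third-person character to the teleport point of another referenced teleporter.
; When the character enters Box while active, it deactivates the destination before relocating the character, preventing an immediate bounce back.
; A teleporter becomes active again once the character ends overlap with OuterBox1 and is confirmed absent from that volume.
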(event `self.Box.OnComponentBeginOverlap`
  (params (OverlappedComponent :type "PrimitiveComponent Object Reference") (OtherActor :type "Actor Object Reference") (OtherComp :type "PrimitiveComponent Object Reference") (OtherBodyIndex :type Integer) (bFromSweep :type Boolean) (SweepResult :type "HitResult Structure (by ref)"))
  (if (`self.bIsActive`)
    (bind _asbp_third_person_character (cast `/Game/ThirdPerson/Blueprints/BP_ThirdPersonCharacter` OtherActor))
    (bind _teleport (`self.Teleport`)
      (:`then`
        (set `/Game/BossFightProject/Core/BP_Teleport.bIsActive` false _teleport)
        (`self.K2_SetActorLocation` _asbp_third_person_character (`SceneComponent.K2_GetComponentLocation` (`/Game/BossFightProject/Core/BP_Teleport.TeleportPoint` _teleport)) false true))
      (:`else`))))

(event `self.OuterBox1.OnComponentEndOverlap`
  (params (OverlappedComponent :type "PrimitiveComponent Object Reference") (OtherActor :type "Actor Object Reference") (OtherComp :type "PrimitiveComponent Object Reference") (OtherBodyIndex :type Integer))
  (bind _asbp_third_person_character (cast `/Game/ThirdPerson/Blueprints/BP_ThirdPersonCharacter` OtherActor))
  (if (== (`KismetArrayLibrary.Array_Find` (`PrimitiveComponent.GetOverlappingActors` (`self.OuterBox1`) "/Game/ThirdPerson/Blueprints/BP_ThirdPersonCharacter.BP_ThirdPersonCharacter_C") _asbp_third_person_character) -1)
    (set `self.bIsActive` true)))

(fn `UserConstructionScript`)