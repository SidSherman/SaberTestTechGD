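; Boss fight game state that relays player death, boss start and defeat, boss HP changes and pause toggling through event dispatchers.
; Death reloads the current level after a short delay, and GamePause toggles the paused state.
; Boss activation fades in intro music, then a duration-based timer crossfades into a repeatedly respawned loop track.
; Boss death fades out the music and clears that timer.
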(event `Death`
  (`self.OnDeath`)
  (`KismetSystemLibrary.Delay` 3.0)
  (bind _returnvalue (`GameplayStatics.GetCurrentLevelName` true))
  (`GameplayStatics.OpenLevel` (`KismetStringLibrary.Conv_StringToName` _returnvalue)))

(event `BossDeath`
  (`self.OnBoss` true)
  (bind _musicloop (`self.MusicLoop`)
    (:`then`
      (`AudioComponent.FadeOut` _musicloop 3.0 0.0 "Linear")
      (`AudioComponent.StopDelayed` _musicloop 3.0))
    (:`else`
      _))
  (`KismetSystemLibrary.K2_ClearAndInvalidateTimerHandle` (`self.MusciTimer`)))

(event `BossActive`
  (`self.OnBoss` false)
  (`self.PlayMusic` (`self.MusicStart`)))

(event `PlayMusic`
  (params (Sound :type "SoundBase Object Reference"))
  (bind _returnvalue (`GameplayStatics.SpawnSound2D` Sound 1.0 1.0 0.0 null))
  (set `self.MusicLoop` _returnvalue)
  (`AudioComponent.FadeIn` _returnvalue 1.0 1.0 0.0 "Linear")
  (bind _returnvalue_2 (`KismetSystemLibrary.K2_SetTimerDelegate` (delegate `MusicLoopTimer`) (`SoundBase.Duration` Sound)))
  (set `self.MusciTimer` _returnvalue_2))

(event `MusicLoopTimer`
  (`AudioComponent.FadeOut` (stale `PlayMusic` _returnvalue) 1.0 0.0 "Linear")
  (`self.PlayMusic` "/Game/BossFightProject/Music/A_Battle_Music_for_Dungeons___Dragons___Музыка_Схваток_и_Сражений_для_ДнД_Loop.A_Battle_Music_for_Dungeons___Dragons___Музыка_Схваток_и_Сражений_для_ДнД_Loop"))

(event `BossHPChange`
  (params (HP :type "Float (double-precision)") (MAxHP :type "Float (double-precision)"))
  (`self.OnBossHPChange` HP MAxHP))

(event `GamePause`
  (if (`GameplayStatics.IsGamePaused`)
    (`GameplayStatics.SetGamePaused` false)
    (`self.OnGamePaused` false)
    (else
      (`GameplayStatics.SetGamePaused` true)
      (`self.OnGamePaused` true))))

(fn `UserConstructionScript`)