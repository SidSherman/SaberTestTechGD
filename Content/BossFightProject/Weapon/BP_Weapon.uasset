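; Hitscan weapon for the third-person player character, handling firing, ammo, fire-rate timing and reload state.
; Shots trace from the follow camera with random aim or hip spread, applying damage, sparks and decals.
; The barrel is re-aimed to launch a cosmetic tracer whose lifespan matches impact distance, alongside muzzle flash, sound and camera shake.
; A separate fake spread grows per shot, eases back on Tick and is broadcast through a dispatcher.
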(event `self.ReceiveTick`
  (params (DeltaSeconds :type "Float (single-precision)"))
  (bind _fakespreading (`self.FakeSpreading`))
  (bind _returnvalue (`KismetMathLibrary.SelectFloat` (`self.AimSpreading`) (`self.Spreading`) (`self.bIsAiming`)))
  (if (not (`KismetMathLibrary.NearlyEqual_FloatFloat` _fakespreading _returnvalue))
    (bind _output_get (set `self.FakeSpreading` (`KismetMathLibrary.FInterpTo_Constant` _fakespreading _returnvalue DeltaSeconds (`self.SpreadingInterpSpeed`))))
    (`self.OnSpreadingChange` _output_get)))

(event `self.Shoot`
  (bind _returnvalue_location (`KismetMathLibrary.BreakTransform` (`SceneComponent.K2_GetComponentToWorld` (`self.Barrel`))))
  (bind _returnvalue_location_2 (`KismetMathLibrary.BreakTransform` (`SceneComponent.K2_GetComponentToWorld` (`self.Barrel`))))
  (bind _returnvalue (`KismetMathLibrary.Vector_Distance` (`self.ResultImpactPoint`) _returnvalue_location_2))
  (bind _bhasammo (`self.HasAmmo`))
  (if _bhasammo
    (`self.CalculateOffset`)
    (`self.UpdateBarrelTransfotmForRealShoot`)
    ;[1 1 1] HitScan
    (bind _outhit (`KismetSystemLibrary.LineTraceSingle` (`SceneComponent.K2_GetComponentLocation` (`AleksandrLaskusTestTCharacter.FollowCamera` (`self.PlayerWeaponOwner`))) (`self.CameraImpactPoint`) "TraceTypeQuery3"))
    (if (`GameplayStatics.BreakHitResult` _outhit)
      (`GameplayStatics.ApplyDamage` (`.HitActor` (`GameplayStatics.BreakHitResult` _outhit)) (`self.Base Damage`) (`self.GetInstigatorController`) self)
      (`GameplayStatics.SpawnEmitterAtLocation` "/Game/RedneckChan_XYZ_GD/Weapons/VFX/InfinityBladeEffects/Effects/FX_Combat_Base/Impact/P_ImpactSpark.P_ImpactSpark" (`.Location` (`GameplayStatics.BreakHitResult` _outhit)) (`KismetMathLibrary.FindLookAtRotation` (`.Location` (`GameplayStatics.BreakHitResult` _outhit)) (`SceneComponent.K2_GetComponentLocation` (`AleksandrLaskusTestTCharacter.FollowCamera` (`self.PlayerWeaponOwner`)))) (0.2 0.2 0.2))
      (`|SpawnActorFromClass` "/Game/_Kitties/Weapon/Effects/Decals/Images/BP_Decal.BP_Decal_C" (`KismetMathLibrary.MakeTransform` (`.Location` (`GameplayStatics.BreakHitResult` _outhit)) (`KismetMathLibrary.Conv_VectorToRotator` (`.Normal` (`GameplayStatics.BreakHitResult` _outhit)))) "AlwaysSpawn" "OverrideRootScale" null null))
    (`GameplayStatics.PlaySoundAtLocation` "/Game/Dev/ContentToDelete/Weapon/Sounds/Pistol/A_colt-smg-Fire_1_Cue.A_colt-smg-Fire_1_Cue" _returnvalue_location (struct) 0.5 1.0 0.0 null null null null)
    (`self.UpdateBarrelTransfotmForFakeShoot`)
    (if (not (< _returnvalue 100.0))
      ;[1 1 1] CheckDistance to ImpactPoint Nad Spawn Fake Trace
      (bind _returnvalue_2 (`|SpawnActorFromClass` "/Game/BossFightProject/Weapon/BP_FakeTraceProjectile.BP_FakeTraceProjectile_C" (`SceneComponent.K2_GetComponentToWorld` (`self.Barrel`)) "AlwaysSpawn" "OverrideRootScale" null (`self.GetInstigator`)))
      (`self.SetLifeSpan` _returnvalue_2 (/ _returnvalue (`MovementComponent.GetMaxSpeed` (`/Game/BossFightProject/Weapon/BP_Projectile.ProjectileMovement` _returnvalue_2)))))
    (`SceneComponent.K2_SetRelativeLocationAndRotation` :`self` (`self.Barrel`))
    (`GameplayStatics.SpawnEmitterAttached` "/Game/PrototypeWeap/FX/P_Pistol_MuzzleFlash.P_Pistol_MuzzleFlash" (`self.Barrel`) "None" (0.0 0.0 0.0) (struct) (1.0 1.0 1.0) "SnapToTarget")
    (set `self.bIsShooting` true)
    (bind _returnvalue_3 (`KismetSystemLibrary.K2_SetTimerDelegate` (delegate `AllowShoot`) (`self.ShootingRate`)))
    (set `self.ShootingTimerHandler` _returnvalue_3)
    (`/Engine/EditorBlueprintResources/StandardMacros.DecrementInt` (`self.Ammo`)
      (:`  `
        (`LegacyCameraShake.StartLegacyCameraShake` (`GameplayStatics.GetPlayerCameraManager` 0) (`self.Shake Class`))
        (bind _output_get (set `self.FakeSpreading` (`KismetMathLibrary.FClamp` (+ (`self.FakeSpreading`) (`self.SpreadingIncrement`)) 0.0 (`self.MaxFakeSpreading`))))
        (`self.OnSpreadingChange` _output_get)))
    (else
      (`GameplayStatics.PlaySoundAtLocation` "/Game/Dev/ContentToDelete/Weapon/Sounds/AssultRifle/A_Empty_Shot_Cue.A_Empty_Shot_Cue" (`self.K2_GetActorLocation`) (struct) 1.0 1.0 0.0 null null null null))))

(event `self.ReceiveBeginPlay`
  (set `self.Ammo` (`self.MaxAmmo`))
  (bind _asbp_third_person_character (cast `/Game/ThirdPerson/Blueprints/BP_ThirdPersonCharacter` (`self.GetOwner`)))
  (set `self.PlayerWeaponOwner` _asbp_third_person_character)
  (set `self.Spreading` (`self.Spreading`)))

(event `AllowShoot`
  (`KismetSystemLibrary.K2_ClearAndInvalidateTimerHandle` (`self.ShootingTimerHandler`))
  (set `self.bIsShooting` false))

(event `self.CancelReload`
  ;[1 1 1] Reload Logic
  (set `self.bIsReloading` false))

(event `self.StartReload`
  ;[1 1 1] Reload Logic
  (set `self.bIsReloading` true))

(event `self.FinishReload`
  ;[1 1 1] Reload Logic
  (set `self.Ammo` (`self.MaxAmmo`))
  (set `self.bIsReloading` false)
  (`self.OnFInishReload` (`self.MaxAmmo`) (`self.Ammo`)))

(fn `CalculateOffset`
  (bind _returnvalue (`KismetMathLibrary.SelectFloat` (`self.AimSpreading`) (`self.Spreading`) (`self.bIsAiming`)))
  (bind _followcamera (`AleksandrLaskusTestTCharacter.FollowCamera` (`self.PlayerWeaponOwner`)))
  (set `self.CameraImpactPoint` (+ (+ (`SceneComponent.K2_GetComponentLocation` _followcamera) (* (`SceneComponent.GetForwardVector` _followcamera) 2000.0)) (`KismetMathLibrary.MakeVector` (`KismetMathLibrary.RandomFloatInRange` (* _returnvalue -1.0) _returnvalue) (`KismetMathLibrary.RandomFloatInRange` (* _returnvalue -1.0) _returnvalue) (`KismetMathLibrary.RandomFloatInRange` (* _returnvalue -1.0) _returnvalue)))))

(fn `CanShoot`
  (returns (bCanShoot :type Boolean))
  (return (not (`self.bIsShooting`))))

(fn `HasAmmo`
  (returns (bHasAmmo :type Boolean))
  (return (> (`self.Ammo`) 0)))

(fn `IsFullAmmo`
  (returns (bIsFullAmmo :type Boolean))
  (return false))

(fn `IsReloading`
  (returns (bIsReloading :type Boolean))
  (return (`self.bIsReloading`)))

(fn `UpdateBarrelTransfotmForFakeShoot`
  (bind _barrel (`self.Barrel`))
  (bind _returnvalue_location (`KismetMathLibrary.BreakTransform` (`SceneComponent.K2_GetComponentToWorld` (`self.Barrel`))))
  (bind _outhit (`KismetSystemLibrary.LineTraceSingle` (`SceneComponent.K2_GetComponentLocation` (`AleksandrLaskusTestTCharacter.FollowCamera` (`self.PlayerWeaponOwner`))) (`self.CameraImpactPoint`) "TraceTypeQuery3"))
  (bind _returnvalue (`KismetMathLibrary.SelectVector` (`.Location` (`GameplayStatics.BreakHitResult` _outhit)) (`self.CameraImpactPoint`) (`GameplayStatics.BreakHitResult` _outhit)))
  (set `self.ResultImpactPoint` _returnvalue)
  (`SceneComponent.K2_SetRelativeLocation` _barrel (0.0 0.0 0.0) false false)
  (`SceneComponent.K2_SetWorldRotation` _barrel (`KismetMathLibrary.FindLookAtRotation` _returnvalue_location _returnvalue) false false))

(fn `UpdateBarrelTransfotmForRealShoot`
  (bind _barrel (`self.Barrel`))
  (bind _barrel_2 (`self.Barrel`))
  (bind _returnvalue (`SceneComponent.K2_GetComponentLocation` _barrel))
  (bind _returnvalue_location (`KismetMathLibrary.BreakTransform` (`SceneComponent.K2_GetComponentToWorld` (`self.Barrel`))))
  (bind _returnvalue_2 (`SceneComponent.K2_GetComponentLocation` (`AleksandrLaskusTestTCharacter.FollowCamera` (`self.PlayerWeaponOwner`))))
  (bind _outhit (`KismetSystemLibrary.LineTraceSingle` _returnvalue_2 (`self.CameraImpactPoint`) "TraceTypeQuery3"))
  (bind _returnvalue_3 (`KismetMathLibrary.SelectVector` (`.Location` (`GameplayStatics.BreakHitResult` _outhit)) (`self.CameraImpactPoint`) (`.bInitialOverlap` (`GameplayStatics.BreakHitResult` _outhit))))
  (bind (_t _intersection _returnvalue_4) (`KismetMathLibrary.LinePlaneIntersection_OriginNormal` _returnvalue_2 _returnvalue_3 _returnvalue (`SceneComponent.GetForwardVector` _barrel)))
  (`SceneComponent.K2_SetWorldLocation` _barrel_2 (`KismetMathLibrary.SelectVector` _intersection _returnvalue _returnvalue_4) false false)
  (`SceneComponent.K2_SetWorldRotation` _barrel_2 (`KismetMathLibrary.FindLookAtRotation` _returnvalue_location _returnvalue_3) false false))

(fn `UserConstructionScript`)