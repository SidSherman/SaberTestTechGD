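; Homing projectile that steers toward a Target actor and can be destroyed by damage from an opposing controller.
; After a launch delay, a looping timer lerps rotation toward the target and resets velocity along that heading at max speed.
; RotationSpeed is the timer interval, while RotationAlpha sets each step's turn strength.
; Overlap handling defers to the parent class, and destruction plays an impact sound and sparkle effect.
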(event `self.ReceiveBeginPlay`
  (`parent.ReceiveBeginPlay`)
  (`KismetSystemLibrary.Delay` (`self.HomingDelay`))
  (bind _returnvalue (`KismetSystemLibrary.K2_SetTimerDelegate` (delegate `RotateToTargetTick`) (`self.RotationSpeed`) true))
  (set `self.RotationTimerHandle` _returnvalue))

(event `RotateToTargetTick`
  (bind (_returnvalue_x _returnvalue_y _returnvalue_z) (`KismetMathLibrary.BreakVector` (`self.K2_GetActorLocation`)))
  (bind _projectilemovement (`self.ProjectileMovement`))
  (bind _target (`self.Target`)
    (:`then`
      (bind (_returnvalue_x_2 _returnvalue_y_2 _returnvalue_z_2) (`KismetMathLibrary.BreakVector` (`self.K2_GetActorLocation` _target)))
      (bind _returnvalue (`KismetMathLibrary.RLerp` (`self.K2_GetActorRotation`) (`KismetMathLibrary.FindLookAtRotation` (`KismetMathLibrary.MakeVector` _returnvalue_x _returnvalue_y _returnvalue_z) (`KismetMathLibrary.MakeVector` _returnvalue_x_2 _returnvalue_y_2 _returnvalue_z_2)) (`self.RotationAlpha`) true))
      (`self.K2_SetActorRotation` _returnvalue)
      (set `MovementComponent.Velocity` (* (`KismetMathLibrary.GetForwardVector` _returnvalue) (`MovementComponent.GetMaxSpeed` _projectilemovement)) _projectilemovement))
    (:`else`)))

(event `self.ReceiveActorBeginOverlap`
  (params (OtherActor :type "Actor Object Reference"))
  (`parent.ReceiveActorBeginOverlap` OtherActor))

(event `self.ReceiveAnyDamage`
  (params (Damage :type "Float (single-precision)") (DamageType :type "DamageType Object Reference") (InstigatedBy :type "Controller Object Reference") (DamageCauser :type "Actor Object Reference"))
  (`/Engine/EditorBlueprintResources/StandardMacros.IsValid` InstigatedBy
    (:`Is Valid`
      (if (!= InstigatedBy (`self.GetInstigatorController`))
        (`self.K2_DestroyActor`)))))

(event `self.ReceiveDestroyed`
  (bind _returnvalue (`self.K2_GetActorLocation`))
  (`GameplayStatics.PlaySoundAtLocation` "/Game/Dev/ContentToDelete/Weapon/SciFiWeapLight/Sound/Knife/Knife_ImpactBody_Cue.Knife_ImpactBody_Cue" _returnvalue (struct) 0.5 1.0 0.0 null null null null)
  (`GameplayStatics.SpawnEmitterAtLocation` "/Game/Dev/ContentToDelete/Realistic_Starter_VFX_Pack_Vol2/Particles/Explosion/P_Explosion_Sparcle.P_Explosion_Sparcle" _returnvalue (struct) (0.5 0.5 0.5)))

(fn `UserConstructionScript`
  (`parent.UserConstructionScript`))