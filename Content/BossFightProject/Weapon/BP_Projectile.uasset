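; BP_Projectile is a weapon projectile Actor that damages what it overlaps and expires after a configurable lifespan.
; Overlaps with BPI_Projectile implementers are ignored; any other overlap destroys the projectile.
; Damage is applied first unless the other actor's instigator, or the actor itself when it has none, matches the projectile's instigator, avoiding self-hits.
; A CanBlock function exposes whether the projectile is blockable.
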(event `self.ReceiveBeginPlay`
  (`self.SetLifeSpan` (`self.InitialLifeSpan`)))

(event `self.ReceiveActorBeginOverlap`
  (params (OtherActor :type "Actor Object Reference"))
  (bind _returnvalue (`self.GetInstigator` OtherActor))
  (bind _returnvalue_2 (`self.GetInstigator`))
  (cast `/Game/BossFightProject/Weapon/BPI_Projectile` OtherActor
    (:`CastFailed`
      (`/Engine/EditorBlueprintResources/StandardMacros.IsValid` _returnvalue
        (:`Is Valid`
          (if (!= _returnvalue _returnvalue_2)
            (`GameplayStatics.ApplyDamage` OtherActor (`self.Base Damage`) (`self.GetInstigatorController`) self :!label _label)
            (`self.K2_DestroyActor`)
            (else
              (`self.K2_DestroyActor` :!label _label_2))))
        (:`Is Not Valid`
          (if (!= OtherActor _returnvalue_2)
            (goto _label)
            (else
              (goto _label_2))))))))

(fn `CanBlock`
  (returns (bValue :type Boolean))
  (return (`self.bCanBlock`)))

(fn `UserConstructionScript`)